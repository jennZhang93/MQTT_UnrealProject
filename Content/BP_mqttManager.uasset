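; BP_mqttManager is an MQTT messaging manager that links the game to a broker and passes received messages to the HUD.
; BeginPlay creates the client from the configured server IP, while Connect, Subscribe and Send are separate events that drive it.
; Subscribe stores the topic, which Send reuses for publishing.
; Callbacks print connection, subscription, send and receive status on screen.
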(event `Connect`
  (`MqttClientInterface.Connect` (`self.client_ref`) (make `MqttConnectionData` "") (delegate `onconnect`)))

(event `self.ReceiveBeginPlay`
  (`KismetSystemLibrary.PrintString` "Hello")
  (bind _returnvalue (`MqttUtilitiesBPL.CreateMqttClient` (make `MqttClientConfig` (`self.server_ip`) 1883 "unrealmqtt")))
  (set `self.client_ref` _returnvalue))

(event `onconnect`
  (`KismetSystemLibrary.PrintString` "connect!" true true (struct :`R` 0.989583 :`B` 0.320625 :`A` 1.0) 20.0))

(event `Subscribe`
  (params (topic :type String))
  (set `self.topic` topic)
  (`MqttClientInterface.Subscribe` (`self.client_ref`) (`self.topic`) 0)
  (`MqttClientInterface.SetOnSubscribeHandler` (`self.client_ref`) (delegate `on sub`))
  (`MqttClientInterface.SetOnMessageHandler` (`self.client_ref`) (delegate `on msg`)))

(event `on msg`
  (params (message :type "MqttMessage Structure"))
  (`KismetSystemLibrary.PrintString` (`KismetStringLibrary.Concat_StrStr` "msg received: " message_Message) true true (struct :`R` 0.989583 :`B` 0.320625 :`A` 1.0) 20.0)
  (`/Game/WBP_mqttSend.Msg recv` (`self.hud`) message_Message))

(event `on sub`
  (params (mid :type Integer) (qos :type "Array of Integer (by ref)"))
  (`KismetSystemLibrary.PrintString` (`KismetStringLibrary.Concat_StrStr` "subscribe succeed" (`KismetStringLibrary.Conv_IntToString` mid)) true true (struct :`R` 0.989583 :`B` 0.320625 :`A` 1.0) 20.0))

(event `Send`
  (params (msg :type String))
  (bind _client_ref (`self.client_ref`))
  (`MqttClientInterface.Publish` _client_ref (make `MqttMessage` "" msg _ (`self.topic`)))
  (`MqttClientInterface.SetOnPublishHandler` _client_ref (delegate `on publish`)))

(event `on publish`
  (params (mid :type Integer))
  (`KismetSystemLibrary.PrintString` (`KismetStringLibrary.Concat_StrStr` "msg sent: " (stale `Send` msg)) true true (struct :`R` 0.989583 :`B` 0.320625 :`A` 1.0) 20.0))

(fn `UserConstructionScript`)